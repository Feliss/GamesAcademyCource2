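; BP_WeaponBase is a base weapon component that deals overlap-based damage through a static mesh attached as its first child.
; On BeginPlay it caches that mesh, sets its collision channel, binds its overlap event, disables damage and ignores the owner when moving.
; ActivateDamage and DeactivateDamage toggle the mesh between query-only and no collision.
; Each overlap applies fixed damage with the owner as causer.
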(event Custom|Initialize
  (bind _asstatic_mesh_component (Utilities|Casting|CastToStaticMeshComponent (Components|GetChildComponent self 0))
    (:then
      (Variables|Default|SetMainMesh _asstatic_mesh_component)
      (Collision|SetCollisionEnabled (Variables|Default|GetMainMesh) "QueryOnly")
      (Collision|SetCollisionObjectType (Variables|Default|GetMainMesh) "ECC_GameTraceChannel1")
      (Collision|AssignOnComponentBeginOverlap (Variables|Default|GetMainMesh) (delegate Custom|OnComponentBeginOverlap_Event_0))
      (CallFunction|DeactivateDamage))
    (:CastFailed
      (Development|PrintString "Weapon is not Static Mesh Component!!! " true true "(R=1.000000,G=0.078098,B=0.000000,A=1.000000)"))))

(event Custom|OnComponentBeginOverlap_Event_0
  (params (OverlappedComponent :type Primitive%20Component%20Object%20Reference) (OtherActor :type Actor%20Object%20Reference) (OtherComp :type Primitive%20Component%20Object%20Reference) (OtherBodyIndex :type Integer) (bFromSweep :type Boolean) (SweepResult :type Hit%20Result%20Structure%20%28by%20ref%29))
  (Game|Damage|ApplyDamage OtherActor 3e+01 0 (Components|GetOwner)))

(event EventBeginPlay
  (CallFunction|Initialize)
  (Collision|IgnoreActorwhenMoving (Variables|Default|GetMainMesh) (Components|GetOwner) true))

(event EventTick
  (params (DeltaSeconds :type Float%20%28single-precision%29)))

(fn ActivateDamage
  (Collision|SetCollisionEnabled (Variables|Default|GetMainMesh) "QueryOnly"))

(fn DeactivateDamage
  (Collision|SetCollisionEnabled (Variables|Default|GetMainMesh) "NoCollision"))