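; Camera shake effect for strikes that rotates the camera with a differently randomized strength each time it plays.
; On PlayShake it overwrites the pitch and yaw rotation oscillators with Perlin noise waveforms at a fixed frequency.
; RandomAmplitude supplies each axis with a random magnitude and random sign, keeping the amplitude away from zero in either direction.
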(event EventPlayShake
  (params (Scale :type Float%20%28single-precision%29))
  (bind _returnvalue (Math|Float|MakeLiteralFloat 4.0))
  (Utilities|Struct|SetmembersinROscillator (Variables|Default|GetRotOscillation) (Utilities|Struct|MakeFOscillator (CallFunction|RandomAmplitude) _returnvalue "PerlinNoise") (Utilities|Struct|MakeFOscillator (CallFunction|RandomAmplitude) _returnvalue "PerlinNoise")))

(fn RandomAmplitude
  (bind _returnvalue (Math|Random|RandomFloatinRange 1.0 2.0))
  (return (Math|Float|SelectFloat (* _returnvalue -1.0) _returnvalue (Math|Random|RandomBool))))