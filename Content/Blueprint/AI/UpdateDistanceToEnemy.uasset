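; Behavior tree service that keeps a blackboard value updated with the AI's distance to its enemy.
; On activation and on each tick, it casts the owner to an AIController and measures from the controlled pawn to the BBEnemy actor.
; The result is written as a float to the BBDistance key.
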(event EventTick
  (params (OwnerActor :type Actor%20Object%20Reference) (DeltaSeconds :type Float%20%28single-precision%29))
  (Variables|Default|SetOwnerActor OwnerActor)
  (bind _asaicontroller (Utilities|Casting|CastToAIController (Variables|Default|GetOwnerActor)))
  (Class|BTFunctionLibrary|SetBlackboardValueasFloat (Variables|Default|GetBBDistance) (Transformation|GetDistanceTo (Pawn|GetControlledPawn _asaicontroller) (AI|BehaviorTree|GetBlackboardValueasActor (Variables|Default|GetBBEnemy)))))

(event EventReceiveActivation
  (params (OwnerActor :type Actor%20Object%20Reference))
  (Variables|Default|SetOwnerActor OwnerActor)
  (bind _asaicontroller (Utilities|Casting|CastToAIController (Variables|Default|GetOwnerActor)))
  (Class|BTFunctionLibrary|SetBlackboardValueasFloat (Variables|Default|GetBBDistance) (Transformation|GetDistanceTo (Pawn|GetControlledPawn _asaicontroller) (AI|BehaviorTree|GetBlackboardValueasActor (Variables|Default|GetBBEnemy)))))