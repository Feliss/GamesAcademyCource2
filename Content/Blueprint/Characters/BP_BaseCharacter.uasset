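; Base player character with switchable first/third-person cameras, camera-relative movement, zoom, sprint, melee combat and an inventory.
; Strike montages toggle weapon damage through notifies, with power strikes advancing a three-stage combo that resets after a short delay.
; Overlapped Item actors are added to the inventory; dropping async-loads the item class and spawns it with physics ahead.
; Damage events destroy the character at zero hit points, and number keys add or drop test items.
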(event OnComponentBeginOverlap(Capsule)
  (params (OverlappedComponent :type Primitive%20Component%20Object%20Reference) (OtherActor :type Actor%20Object%20Reference) (OtherComp :type Primitive%20Component%20Object%20Reference) (OtherBodyIndex :type Integer) (bFromSweep :type Boolean) (SweepResult :type Hit%20Result%20Structure%20%28by%20ref%29))
  (bind _asitem (Utilities|Casting|CastToItem OtherActor))
  (CallFunction|AddItemActortoInventory _asitem))

(event Custom|DropFromInventory
  (params (Item :type Item%20Data%20Asset%20Object%20Reference))
  (bind _success (Default|RemoveItem (Variables|Default|GetInventory) Item 1))
  (if _success
    (bind _class (Utilities|AsyncLoadClassAsset (Variables|/Script/SuperRpg.ItemDataAsset|GetActorToUse Item))
      (:Completed
        (bind _asitem (Utilities|Casting|CastToItemClass _class))
        (bind _returnvalue (Game|SpawnActorfromClass _asitem (Math|Transform|MakeTransform (+ (Transformation|GetActorLocation) (* (Transformation|GetActorForwardVector) 1.4e+02)) (Math|Random|RandomRotator true)) "AdjustIfPossibleButAlwaysSpawn" 0 Item 0))
        (Utilities|IsValid _returnvalue
          (:Is%20Valid
            (Physics|SetSimulatePhysics (Variables|/Game/Blueprint/Items/Item.Item_C|GetStaticMesh _returnvalue) true)))))))

(event Custom|AddToInventory
  (params (Item :type Item%20Data%20Asset%20Object%20Reference))
  (Default|AddItem (Variables|Default|GetInventory) Item 1))

(event Custom|AddItemActorToInventory
  (params (ItemActor :type Item%20Object%20Reference))
  (CallFunction|AddtoInventory (Variables|/Game/Blueprint/Items/Item.Item_C|GetAsset ItemActor))
  (Actor|DestroyActor ItemActor))

(event EventBeginPlay)

(event Collision|EventActorBeginOverlap
  (params (OtherActor :type Actor%20Object%20Reference)))

(event EventTick
  (params (DeltaSeconds :type Float%20%28single-precision%29)))

(event EventOnTakeDamage
  (params (TotalHitPoints :type Float%20%28single-precision%29))
  (Development|PrintString (Utilities|String|ToString(Float) TotalHitPoints))
  (if (<= TotalHitPoints 0.0)
    (Actor|DestroyActor)))

(event Input|ActionEvents|InputActionZoomForward
  (params (Key :type Key%20Structure :default "None"))
  (bind _springarm (Variables|Default|GetSpringArm))
  (:Pressed
    (Variables|/Script/Engine.SpringArmComponent|SetTargetArmLength _springarm (+ (Variables|/Script/Engine.SpringArmComponent|GetTargetArmLength _springarm) -4e+01))))

(event Input|ActionEvents|InputActionStrike
  (params (Key :type Key%20Structure :default "None"))
  (bind _bp_weaponbase (Variables|Default|GetBP_WeaponBase))
  (:Pressed
    (bind _notifyname (Animation|Montage|PlayMontage (Variables|Character|GetMesh) "/Game/Animation/Characters/Zombie/AM_Zombie_Strike.AM_Zombie_Strike" 1.2 0.0 "FastStrike")
      (:OnNotifyBegin
        (switch name _notifyname
          (:ApplyingDamage
            (Default|ActivateDamage _bp_weaponbase))))
      (:OnNotifyEnd
        (switch name "None"
          (:ApplyingDamage
            (Default|DeactivateDamage _bp_weaponbase)))))))

(event Input|ActionEvents|InputActionZoomBackward
  (params (Key :type Key%20Structure :default "None"))
  (bind _springarm (Variables|Default|GetSpringArm))
  (:Pressed
    (Variables|/Script/Engine.SpringArmComponent|SetTargetArmLength _springarm (+ (Variables|/Script/Engine.SpringArmComponent|GetTargetArmLength _springarm) 4e+01))))

(event Input|ActionEvents|InputActionSprint
  (params (Key :type Key%20Structure :default "None"))
  (bind _charactermovement (Variables|Character|GetCharacterMovement))
  (:Pressed
    (Variables|/Script/Engine.CharacterMovementComponent|SetMaxWalkSpeed _charactermovement (+ (Variables|/Script/Engine.CharacterMovementComponent|GetMaxWalkSpeed _charactermovement) (Variables|Default|GetSprintAdditionalSpeed))))
  (:Released
    (Variables|/Script/Engine.CharacterMovementComponent|SetMaxWalkSpeed _charactermovement (+ (Variables|/Script/Engine.CharacterMovementComponent|GetMaxWalkSpeed _charactermovement) (* (Variables|Default|GetSprintAdditionalSpeed) -1.0)))))

(event Input|ActionEvents|InputActionPowerStrike
  (params (Key :type Key%20Structure :default "None"))
  (bind _bp_weaponbase (Variables|Default|GetBP_WeaponBase))
  (:Pressed
    (bind _notifyname (Animation|Montage|PlayMontage (Variables|Character|GetMesh) (Variables|Default|GetMontageStrikeCompo) 1.2 0.0 (Utilities|Select :Index (Variables|Default|GetComboStrikeState) :NewEnumerator0 "Attack1" :NewEnumerator1 "Attack2" :NewEnumerator2 "Attack3"))
      (:then
        (switch name _notifyname :!label _label
          (:ApplyingDamage
            (Default|DeactivateDamage _bp_weaponbase))))
      (:OnNotifyBegin
        (switch name _notifyname
          (:Attack1Finished
            (Variables|Default|SetComboStrikeState "NewEnumerator1")
            (Animation|StopAnimMontage (Variables|Default|GetMontageStrikeCompo) :!label _label_2)
            (Utilities|FlowControl|Delay 0.5)
            (Variables|Default|SetComboStrikeState "NewEnumerator0"))
          (:Attack2Finished
            (Variables|Default|SetComboStrikeState "NewEnumerator2")
            (goto _label_2))
          (:Attack3Finished
            (Variables|Default|SetComboStrikeState "NewEnumerator0")
            (goto _label_2))
          (:ApplyingDamage
            (Default|ActivateDamage _bp_weaponbase))))
      (:OnNotifyEnd
        (goto _label)))))

(event Input|ActionEvents|InputActionInventorySwitch
  (params (Key :type Key%20Structure :default "None"))
  (:Pressed
    (Utilities|FlowControl|FlipFlop
      (:A
        (Class|MainCharacter|ShowInventory))
      (:B
        (Class|MainCharacter|HideInventory)))))

(event Input|AxisEvents|InputAxisForward
  (params (AxisValue :type Float%20%28single-precision%29))
  (Pawn|Input|AddMovementInput (Math|Vector|RotateVector (Math|Vector|MakeVector AxisValue 0.0 0.0) (Math|Rotator|MakeRotator 0.0 0.0 (.Yaw (Math|Rotator|BreakRotator (Pawn|GetControlRotation :!class /Script/Engine.Pawn))))) 1.0 false))

(event Input|AxisEvents|InputAxisRight
  (params (AxisValue :type Float%20%28single-precision%29))
  (Pawn|Input|AddMovementInput (Math|Vector|RotateVector (Math|Vector|MakeVector 0.0 AxisValue 0.0) (Math|Rotator|MakeRotator 0.0 0.0 (.Yaw (Math|Rotator|BreakRotator (Pawn|GetControlRotation :!class /Script/Engine.Pawn))))) 1.0 false))

(event Input|AxisEvents|InputAxisTurnUp
  (params (AxisValue :type Float%20%28single-precision%29))
  (Pawn|Input|AddControllerPitchInput (* AxisValue -1.0)))

(event Input|AxisEvents|InputAxisTurnRight
  (params (AxisValue :type Float%20%28single-precision%29))
  (Pawn|Input|AddControllerYawInput AxisValue))

(event Input|KeyboardEvents|J
  (params (Key :type Key%20Structure :default "None"))
  (:Pressed
    (Utilities|FlowControl|FlipFlop
      (:A
        (Components|Activation|Activate (Variables|Default|GetCameraFPS) false)
        (Components|Activation|Deactivate (Variables|Default|GetCameraTPS)))
      (:B
        (Components|Activation|Activate (Variables|Default|GetCameraTPS) false)
        (Components|Activation|Deactivate (Variables|Default|GetCameraFPS))))))

(event Input|KeyboardEvents|1
  (params (Key :type Key%20Structure :default "None"))
  (:Pressed
    (CallFunction|AddtoInventory "/Game/Data/Items/Apple.Apple")))

(event Input|KeyboardEvents|2
  (params (Key :type Key%20Structure :default "None"))
  (:Pressed
    (CallFunction|AddtoInventory "/Game/Data/Items/Sword.Sword")))

(event Input|KeyboardEvents|3
  (params (Key :type Key%20Structure :default "None"))
  (:Pressed
    (CallFunction|DropfromInventory "/Game/Data/Items/Apple.Apple")))

(event Input|KeyboardEvents|4
  (params (Key :type Key%20Structure :default "None"))
  (:Pressed
    (CallFunction|DropfromInventory "/Game/Data/Items/Sword.Sword")))

(fn ConstructionScript)

(fn GotoShelterinEditor
  (Class|BaseCharacter|GotoShelter))