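; Main character Blueprint that adds a health-driven post-process effect to both its first-person and third-person cameras.
; On BeginPlay it creates a dynamic instance of ExamplePostProcess_Inst and registers it as a full-weight blendable on CameraFPS and CameraTPS.
; After the parent's damage handling, OnTakeDamage sets the material's IntencityAdd parameter to the missing-health fraction, so the value rises as hit points drop.
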(event EventBeginPlay
  (|CallParentFunction)
  (bind _returnvalue (Rendering|Material|CreateDynamicMaterialInstance "/Game/Materials/PostProcess/ExamplePostProcess_Inst.ExamplePostProcess_Inst" "None" "None" :!class /Script/Engine.KismetMaterialLibrary))
  (bind _output_get (Variables|Default|SetPPMat _returnvalue))
  (Rendering|AddorUpdateBlendable (Variables|Default|GetCameraFPS) _output_get 1.0 :!class /Script/Engine.CameraComponent)
  (Rendering|AddorUpdateBlendable (Variables|Default|GetCameraTPS) _output_get 1.0 :!class /Script/Engine.CameraComponent))

(event Collision|EventActorBeginOverlap
  (params (OtherActor :type Actor%20Object%20Reference))
  (|CallParentFunction OtherActor) ; This node is disabled and will not be called.\nDrag off pins to build functionality.
)

(event EventTick
  (params (DeltaSeconds :type Float%20%28single-precision%29))
  (|CallParentFunction DeltaSeconds) ; This node is disabled and will not be called.\nDrag off pins to build functionality.
)

(event EventOnTakeDamage
  (params (TotalHitPoints :type Float%20%28single-precision%29))
  (|CallParentFunction TotalHitPoints)
  (Rendering|Material|SetScalarParameterValue (Variables|Default|GetPPMat) "IntencityAdd" (- 1.0 (/ (Variables|Default|GetHitPoints) (Variables|Default|GetMaxHitPoints))) :!class /Script/Engine.MaterialInstanceDynamic))

(fn ConstructionScript
  (|CallParentFunction))